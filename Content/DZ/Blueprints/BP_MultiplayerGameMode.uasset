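; Multiplayer game mode that splits joining players into two teams.
; On post-login, each BP_PlayerController goes to team 1 only when that team is smaller, otherwise to team 2, receiving the matching team ID.
; Each team is tracked in its own controller array, and logout removes the leaving controller from the array that holds it.
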(event EventBeginPlay)

(event EventTick
  (params (DeltaSeconds :type Float%20%28single-precision%29)))

(event EventPostLogin
  (params (NewPlayer :type Player%20Controller%20Object%20Reference))
  (bind _asbp_player_controller (Utilities|Casting|CastToBP_PlayerController NewPlayer))
  (if (< (Utilities|Array|Length (Variables|Default|GetFirstTeamPC)) (Utilities|Array|Length (Variables|Default|GetSecondTeamPC)))
    (Default|SetTeamID _asbp_player_controller 1)
    (Utilities|Array|Add (Variables|Default|GetFirstTeamPC) _asbp_player_controller)
    (else
      (Default|SetTeamID _asbp_player_controller 2)
      (Utilities|Array|Add (Variables|Default|GetSecondTeamPC) _asbp_player_controller))))

(event EventOnLogout
  (params (ExitingController :type Controller%20Object%20Reference))
  (bind _asbp_player_controller (Utilities|Casting|CastToBP_PlayerController ExitingController))
  (if (Utilities|Array|ContainsItem (Variables|Default|GetFirstTeamPC) _asbp_player_controller)
    (Utilities|Array|RemoveItem (Variables|Default|GetFirstTeamPC) _asbp_player_controller)
    (else
      (Utilities|Array|RemoveItem (Variables|Default|GetSecondTeamPC) _asbp_player_controller))))

(fn ConstructionScript)