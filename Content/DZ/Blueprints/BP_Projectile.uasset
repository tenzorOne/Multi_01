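; Networked projectile that flies straight forward, damages multiplayer pawns it overlaps and explodes.
; The server moves it each tick by teleport-free, unswept location updates and handles overlaps, ignoring itself and its owner.
; Hits pass damage plus the instigator's health component and HP bar to the struck pawn, then multicast the explosion effect.
; A lifetime timer or any valid hit destroys it after a short delay.
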(event OnComponentBeginOverlap(Collision)
  (params (OverlappedComponent :type Primitive%20Component%20Object%20Reference) (OtherActor :type Actor%20Object%20Reference) (OtherComp :type Primitive%20Component%20Object%20Reference) (OtherBodyIndex :type Integer) (bFromSweep :type Boolean) (SweepResult :type Hit%20Result%20Structure%20%28by%20ref%29))
  (if (Networking|IsServer)
    (CallFunction|ServerProjectileHit OtherActor (Transformation|GetActorLocation))))

(event Custom|Server_ProjectileLifeTime
  (Utilities|FlowControl|Delay 0.1)
  (Actor|DestroyActor))

(event Custom|Server_ProjectileMovement
  (Transformation|SetActorLocation (+ (Transformation|GetActorLocation) (* (Transformation|GetActorForwardVector) (* (Utilities|Time|GetWorldDeltaSeconds) (Variables|Default|GetSpeed)))) false false))

(event Custom|Server_ProjectileHit
  (params (OverlappedActor :type Actor%20Object%20Reference) (ProjectileLocation :type Vector))
  (bind _returnvalue (Game|GetInstigator))
  (bind _asbp_multiplayer_pawn (Utilities|Casting|CastToBP_MultiplayerPawn _returnvalue))
  (if (and (!= self OverlappedActor) (!= OverlappedActor (Components|GetOwner)))
    (bind _asbp_multiplayer_pawn_2 (Utilities|Casting|CastToBP_MultiplayerPawn OverlappedActor)
      (:then
        (Default|TakeDamage _asbp_multiplayer_pawn_2 (Variables|Default|GetDamage) (Variables|/Game/DZ/Blueprints/BP_MultiplayerPawn.BP_MultiplayerPawn_C|GetHealthComponent _asbp_multiplayer_pawn) (Variables|/Game/DZ/Blueprints/BP_MultiplayerPawn.BP_MultiplayerPawn_C|GetHPBar _asbp_multiplayer_pawn)))
      (:CastFailed
        _))
    (CallFunction|MulticastSpawnHitEffects ProjectileLocation)
    (CallFunction|ServerProjectileLifeTime)))

(event Custom|SpawnHitEffects
  (params (HitLocation :type Vector))
  (Effects|SpawnEmitteratLocation "/Game/StarterContent/Particles/P_Explosion.P_Explosion" HitLocation))

(event Custom|Multicast_SpawnHitEffects
  (params (HitLocation :type Vector))
  (CallFunction|SpawnHitEffects HitLocation))

(event EventBeginPlay
  (Utilities|Time|SetTimerbyEvent (delegate Custom|Server_ProjectileLifeTime) (Variables|Default|GetLifeTime)))

(event EventTick
  (params (DeltaSeconds :type Float%20%28single-precision%29))
  (if (Networking|IsServer)
    (CallFunction|ServerProjectileMovement)))

(fn ConstructionScript)