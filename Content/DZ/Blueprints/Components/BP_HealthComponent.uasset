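; Health component for multiplayer pawns that stores a Health value and keeps the owner's HP bar in step with it.
; SubtractionHealth lowers Health by a given amount, with no clamping or death handling.
; The Health RepNotify casts the owner to BP_MultiplayerPawn and passes the new value to its HPBar, so other owner types get no bar update.
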(event EventTick
  (params (DeltaSeconds :type Float%20%28single-precision%29)))

(fn OnRepHealth
  (bind _asbp_multiplayer_pawn (Utilities|Casting|CastToBP_MultiplayerPawn (Components|GetOwner)))
  (Default|SetHPBar (Variables|/Game/DZ/Blueprints/BP_MultiplayerPawn.BP_MultiplayerPawn_C|GetHPBar _asbp_multiplayer_pawn) (Variables|Default|GetHealth)))

(fn SubtractionHealth
  (params (Value :type Float%20%28single-precision%29))
  (Variables|Default|SetHealth (- (Variables|Default|GetHealth) Value)))