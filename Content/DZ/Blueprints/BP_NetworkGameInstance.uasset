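; Game instance Blueprint that handles LAN multiplayer sessions: hosting, listing and joining games.
; CreateGame creates a session and, on success, opens Level_01 as a listen server.
; GetGames searches for LAN sessions and only prints each one's name, player count and ping.
; JoinToGame runs its own single-result search and joins what it finds, with failures reported through on-screen prints.
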(event Custom|CreateGame
  (|Session (Game|GetPlayerController 0) 16 true
    (:OnSuccess
      (Game|OpenLevel(byName) "Level_01" true "listen"))
    (:OnFailure
      (Development|PrintString "Create session error!" true true "(R=1.000000,G=0.071069,B=0.000000,A=1.000000)" 5.0))))

(event Custom|GetGames
  (bind _results (|FindSessions (Game|GetPlayerController 0) 20 true)
    (:OnSuccess
      (for _array_element _results
        (Development|PrintString (Utilities|String|Append "Server: " (Class|FindSessionsCallbackProxy|GetServerName _array_element) " 
Players: " (Utilities|String|ToString(Integer) (Class|FindSessionsCallbackProxy|GetCurrentPlayers _array_element)) "/" (Utilities|String|ToString(Integer) (Class|FindSessionsCallbackProxy|GetMaxPlayers _array_element)) " 
Ping: " (Utilities|String|ToString(Integer) (Class|FindSessionsCallbackProxy|GetPinginMs _array_element))) true true "(R=0.000000,G=0.660000,B=1.000000,A=1.000000)" 8.0)))
    (:OnFailure
      (Development|PrintString "Current games not found." true true "(R=1.000000,G=0.071069,B=0.000000,A=1.000000)" 5.0))))

(event Custom|JoinToGame
  (bind _returnvalue (Game|GetPlayerController 0))
  (bind _results (|FindSessions _returnvalue 1 true)
    (:OnSuccess
      (for _array_element _results
        (|JoinSession _returnvalue _array_element
          (:OnFailure
            (Development|PrintString "Join to game error!" true true "(R=1.000000,G=0.071069,B=0.000000,A=1.000000)" 5.0)))))
    (:OnFailure
      (Development|PrintString "Current games not found." true true "(R=1.000000,G=0.071069,B=0.000000,A=1.000000)" 5.0))))